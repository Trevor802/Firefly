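; BP_RockPool is a pooled spawner that rains or scatters BP_Rock actors at random points inside its Box bounds.
; A looping timer spawns rocks while active, and the player BP_Character's switch-rock event toggles that state.
; Each rock gets random rotation and scale.
; Until PoolSize is reached it spawns new rocks with a sound at their average location, then reactivates and repositions existing ones round-robin.
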(event Custom|SpawnRock
  (bind _returnvalue (Math|Random|RandomRotator false))
  (bind _box (Variables|Default|GetBox))
  (bind _minscale (Variables|Default|GetMinScale))
  (bind _maxscale (Variables|Default|GetMaxScale))
  (bind _rocks (Variables|Default|GetRocks))
  (bind (_origin _boxextent) (Collision|GetComponentBounds _box))
  (bind _returnvalue_2 (Math|Random|RandomFloatinRange _minscale _maxscale))
  (bind _returnvalue_3 (Math|Random|RandomPointinBoundingBox _origin _boxextent))
  (bind _returnvalue_4 (* "1.000000,1.000000,1.000000" _returnvalue_2))
  (bind _returnvalue_5 (Math|Transform|MakeTransform _returnvalue_3 _returnvalue _returnvalue_4))
  (if (< (Utilities|Array|Length (Variables|Default|GetRocks)) (Variables|Default|GetPoolSize))
    (bind _returnvalue_6 (Game|SpawnActorfromClass "/Game/Trevor/BP_Rock.BP_Rock_C" _returnvalue_5 "Undefined" 0 0))
    (Utilities|Array|Add _rocks _returnvalue_6)
    (bind _returnvalue_7 (Class|GameplayStatics|GetActorArrayAverageLocation _rocks))
    (Audio|PlaySoundatLocation 0 _returnvalue_7 "0, 0, 0" 1.0 1.0 0.0 0 0 0)
    (else
      (Default|Activate (Utilities|Array|Get(acopy) (Variables|Default|GetRocks) (Variables|Default|GetRockIndex)))
      (Transformation|SetActorTransform (Utilities|Array|Get(acopy) (Variables|Default|GetRocks) (Variables|Default|GetRockIndex)) _returnvalue_5)
      (bind _result (Math|Integer|IncrementInt (Variables|Default|GetRockIndex))
        (:%20%20
          (Variables|Default|SetRockIndex (Math|Integer|%(Integer) _result (Variables|Default|GetPoolSize))))))))

(event Custom|OnSpawnRock
  (if (Variables|Default|GetbActivated)
    (CallFunction|SpawnRock)))

(event Custom|OnSwitchRock
  (Variables|Default|SetbActivated (not (Variables|Default|GetbActivated))))

(event EventBeginPlay
  (bind _asbp_character (Utilities|Casting|CastToBP_Character (Game|GetPlayerCharacter 0)))
  (EventDispatchers|BindEventtoSwitchRock _asbp_character (delegate Custom|OnSwitchRock))
  (Utilities|Time|SetTimerbyEvent (delegate Custom|OnSpawnRock) (Variables|Default|GetSpawnInterval) true))

(fn ConstructionScript)