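; BP_Firefly is a floating pawn that travels along an ordered list of target actors, apparently as a guide for the player character.
; BP_Character entering its sphere starts an AI MoveTo toward the current target.
; Leaving the sphere halts it only if that target's WaitPlayer flag is set, with the last flag covering missing entries.
; GoNextTarget, not called within this Blueprint, advances the index and resumes movement, clamping at the last target.
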(event OnComponentBeginOverlap(Sphere)
  (params (OverlappedComponent :type Primitive%20Component%20Object%20Reference) (OtherActor :type Actor%20Object%20Reference) (OtherComp :type Primitive%20Component%20Object%20Reference) (OtherBodyIndex :type Integer) (bFromSweep :type Boolean) (SweepResult :type Hit%20Result%20Structure%20%28by%20ref%29))
  (Utilities|Casting|CastToBP_Character OtherActor)
  (if (not (Variables|Default|GetbMoving))
    (CallFunction|EnableMovement)))

(event OnComponentEndOverlap(Sphere)
  (params (OverlappedComponent :type Primitive%20Component%20Object%20Reference) (OtherActor :type Actor%20Object%20Reference) (OtherComp :type Primitive%20Component%20Object%20Reference) (OtherBodyIndex :type Integer))
  (Utilities|Casting|CastToBP_Character OtherActor)
  (CallFunction|DisableMovement))

(event Custom|GoNextTarget
  (bind _target (Variables|Default|GetTarget))
  (bind _returnvalue (Utilities|Array|Length _target))
  (bind _result (Math|Integer|IncrementInt (Variables|Default|GetTargetIndex))
    (:%20%20
      (CallFunction|EnableMovement)
      (if (>= _result _returnvalue)
        (Variables|Default|SetTargetIndex (- _returnvalue 1))))))

(event Custom|DisableMovement
  (bind _target (CallFunction|WillWait))
  (if _target
    (Variables|Default|SetbMoving false)
    (Components|Movement|StopMovementImmediately (Variables|Default|GetFloatingPawnMovement))))

(event Custom|EnableMovement
  (Variables|Default|SetbMoving true)
  (bind _actor (CallFunction|GetTarget))
  (AI|AIMoveTo self "0, 0, 0" _actor 5e+01 false
    (:OnSuccess
      (Variables|Default|SetbMoving false))))

(fn ConstructionScript)

(fn GetTarget
  (return (Utilities|Array|Get(acopy) (Variables|Default|GetTarget) (Variables|Default|GetTargetIndex))))

(fn WillWait
  (bind _targetindex (Variables|Default|GetTargetIndex))
  (bind _waitplayer (Variables|Default|GetWaitPlayer))
  (bind _returnvalue (Utilities|Array|Length _waitplayer))
  (if (>= _targetindex _returnvalue)
    (return (Utilities|Array|Get(acopy) _waitplayer (- _returnvalue 1)))
    (else
      (return (Utilities|Array|Get(acopy) _waitplayer _targetindex)))))