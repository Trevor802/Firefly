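; BP_Rock is a physics rock that toggles between active and dormant instead of being destroyed, a pattern suited to object pooling.
; Overlapping a BP_KillZone calls Deactivate, which clears velocities, hides the mesh, disables physics, collision and tick, and resets the actor transform.
; Activate clears velocities again and restores visibility, physics, collision and tick; nothing in this Blueprint calls it.
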(event Custom|Deactivate
  (bind _staticmeshcomponent (Variables|Debug|GetStaticMeshComponent))
  (bind _staticmeshcomponent_2 (Variables|Debug|GetStaticMeshComponent))
  (Class|PrimitiveComponent|SetAllPhysicsLinearVelocity _staticmeshcomponent_2 "0, 0, 0" false)
  (Class|PrimitiveComponent|SetPhysicsAngularVelocityinRadians _staticmeshcomponent_2 "0, 0, 0" false "None")
  (Rendering|SetVisibility _staticmeshcomponent false false)
  (Physics|SetSimulatePhysics _staticmeshcomponent false)
  (Collision|SetCollisionEnabled _staticmeshcomponent "NoCollision")
  (Actor|Tick|SetActorTickEnabled false)
  (Transformation|SetActorTransform (Math|Transform|MakeTransform "0, 0, 0" "0, 0, 0" "1,1,1")))

(event Custom|Activate
  (bind _staticmeshcomponent (Variables|Debug|GetStaticMeshComponent))
  (bind _staticmeshcomponent_2 (Variables|Debug|GetStaticMeshComponent))
  (Class|PrimitiveComponent|SetAllPhysicsLinearVelocity _staticmeshcomponent "0, 0, 0" false)
  (Class|PrimitiveComponent|SetPhysicsAngularVelocityinRadians _staticmeshcomponent "0, 0, 0" false "None")
  (Rendering|SetVisibility _staticmeshcomponent_2 true false)
  (Physics|SetSimulatePhysics _staticmeshcomponent_2 true)
  (Collision|SetCollisionEnabled _staticmeshcomponent_2 "QueryAndPhysics")
  (Actor|Tick|SetActorTickEnabled true))

(event EventBeginPlay)

(event Collision|EventActorBeginOverlap
  (params (OtherActor :type Actor%20Object%20Reference))
  (Utilities|Casting|CastToBP_KillZone OtherActor)
  (CallFunction|Deactivate))

(event EventTick
  (params (DeltaSeconds :type Float%20%28single-precision%29)))

(fn ConstructionScript)