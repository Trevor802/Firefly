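; BP_Character is the player character, able to transform between animal forms and spawning smoke when the form changes.
; A fast-moving BP_Rock hit triggers death, which disables movement and sets a dying flag.
; Kill zone overlap or Respawn input restores the start transform, default animal and movement, then calls the respawn notification.
; It also forwards RockSwitch input to a rock-switch call and exposes camera boom activation.
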(event OnComponentHit(CapsuleComponent)
  (params (HitComponent :type Primitive%20Component%20Object%20Reference) (OtherActor :type Actor%20Object%20Reference) (OtherComp :type Primitive%20Component%20Object%20Reference) (NormalImpulse :type Vector :default "0, 0, 0") (Hit :type Hit%20Result%20Structure%20%28by%20ref%29))
  (bind _asbp_rock (Utilities|Casting|CastToBP_Rock OtherActor))
  (if (> (Math|Vector|VectorLength (Transformation|GetVelocity _asbp_rock)) (Variables|Default|GetDeadVelocity))
    (CallFunction|Die)))

(event Custom|Die
  (Components|Activation|Deactivate (Variables|Character|GetCharacterMovement))
  (Variables|Default|SetbDying true))

(event Custom|Respawn
  (Variables|Default|SetbDying false)
  (Transformation|SetActorTransform (Variables|Default|GetStartTrans))
  (Class|FireflyCharacter|Transformto (Variables|Default|GetDefaultAnimal))
  (Components|Activation|Activate (Variables|Character|GetCharacterMovement) false)
  (Default|CallOnRespawn))

(event Custom|SetCameraActive
  (params (bNewActive :type Boolean))
  (Components|Activation|SetActive (Variables|Default|GetCameraBoom) bNewActive false))

(event EventBeginPlay
  (Variables|Default|SetStartTrans (Transformation|GetActorTransform)))

(event Collision|EventActorBeginOverlap
  (params (OtherActor :type Actor%20Object%20Reference))
  (Utilities|Casting|CastToBP_KillZone OtherActor)
  (CallFunction|Respawn))

(event EventTransformto
  (params (eAnimal :type EAnimal%20Enum :default "Human"))
  (Variables|Default|SetbAnimalEqual (Utilities|Enum|NotEqual(Enum) eAnimal (Class|FireflyCharacter|GetAnimal)))
  (|CallParentFunction eAnimal)
  (if (Variables|Default|GetbAnimalEqual)
    (Niagara|SpawnSystematLocation "/Game/Dun/PS_Smoke.PS_Smoke" (Transformation|GetActorLocation))))

(event Input|ActionEvents|InputActionRespawn
  (params (Key :type Key%20Structure :default "None"))
  (:Pressed
    (CallFunction|Respawn)))

(event Input|ActionEvents|InputActionRockSwitch
  (params (Key :type Key%20Structure :default "None"))
  (:Pressed
    (Default|CallSwitchRock)))

(fn ConstructionScript)